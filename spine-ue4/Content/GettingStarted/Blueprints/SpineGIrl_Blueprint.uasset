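; SpineGirl Blueprint is a Spine skeletal animation example character that plays a looping main animation and blinks at random intervals.
; BeginPlay sets the looping "main" animation on track 0.
; Tick counts down a timer, resets it to a short random delay, and layers a one-shot "blink" on track 1, using Spine's multi-track mixing to combine both animations.
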(event `self.ReceiveBeginPlay`
  ;[1 1 1] When SpineGirl begins playing, we set her "main" animation on track 0
  (`SpineSkeletonAnimationComponent.SetAnimation` (`self.SpineSkeletonAnimation`) 0 "main" true))

(event `self.ReceiveTick`
  (params (DeltaSeconds :type "Float (single-precision)"))
  ;[1 1 1] We mix in the "blink" animation randomly on track 1. Every tick, we check if it's time again to playback the blink animation. If it is, we reset the timer to a random value between 0.5 and 1.5 seconds, ,and play the animation
  (bind _output_get (set `self.Time` (- (`self.Time`) DeltaSeconds)))
  (if (<= _output_get 0.0)
    (set `self.Time` (`KismetMathLibrary.RandomFloatInRange` 0.5 1.5))
    (`SpineSkeletonAnimationComponent.SetAnimation` (`self.SpineSkeletonAnimation`) 1 "blink" false)))

(fn `UserConstructionScript`)