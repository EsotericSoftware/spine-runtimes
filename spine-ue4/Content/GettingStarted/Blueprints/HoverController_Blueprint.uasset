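; Hover controller actor that lets the player move a hoverboard target with the keyboard in what appears to be a Spine skeleton example.
; Tick polls the first player controller for held keys, offsetting the root component along world Z with U/J and world X with K/H at a fixed, frame-rate-independent speed, without sweeping.
; According to the graph comment, a SpineBoneDriver on the actor then moves the skeleton's "hoverboard" bone to the actor's location.
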(event `self.ReceiveTick`
  (params (DeltaSeconds :type "Float (single-precision)"))
  (bind _returnvalue (`GameplayStatics.GetPlayerController` 0))
  (bind _returnvalue_2 (* DeltaSeconds 200.0))
  (bind _defaultsceneroot1 (`self.DefaultSceneRoot1`))
  (bind _defaultsceneroot1_2 (`self.DefaultSceneRoot1`))
  ;[1 1 1] Move the actor each tick depending on which of the U/H/J/K keys are pressed. The SpineBoneDriver on this actor will then
  ; Move the "hoverboard" bone in the seleton to this actor's location.
  (`|ExecutionSequence`
    (:`then_0`
      (if (> (`PlayerController.GetInputKeyTimeDown` _returnvalue "U") 0.0)
        (`SceneComponent.K2_AddWorldOffset` _defaultsceneroot1 (`KismetMathLibrary.MakeVector` 0.0 0.0 _returnvalue_2) false false)))
    (:`then_1`
      (if (> (`PlayerController.GetInputKeyTimeDown` _returnvalue "J") 0.0)
        (`SceneComponent.K2_AddWorldOffset` _defaultsceneroot1 (`KismetMathLibrary.MakeVector` 0.0 0.0 (* _returnvalue_2 -1.0)) false false)))
    (:`then_2`
      (if (> (`PlayerController.GetInputKeyTimeDown` _returnvalue "K") 0.0)
        (`SceneComponent.K2_AddWorldOffset` _defaultsceneroot1_2 (`KismetMathLibrary.MakeVector` _returnvalue_2) false false)))
    (:`then_3`
      (if (> (`PlayerController.GetInputKeyTimeDown` _returnvalue "H") 0.0)
        (`SceneComponent.K2_AddWorldOffset` _defaultsceneroot1_2 (`KismetMathLibrary.MakeVector` (* _returnvalue_2 -1.0)) false false)))))

(fn `UserConstructionScript`)