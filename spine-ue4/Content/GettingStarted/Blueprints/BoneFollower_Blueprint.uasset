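; Demo actor Blueprint that toggles the Use Component Transform setting on its Spine bone follower component at runtime.
; On BeginPlay it enables input from the first player controller.
; Left mouse button and space bar share one branch that flips the flag and prints the new value on screen.
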(event `self.ReceiveBeginPlay`
  ;[1 1 1] Enable input with the begining of the level
  (`self.EnableInput` (`GameplayStatics.GetPlayerController` 0)))

(event `Key|LeftMouseButton`
  (params (Key :type "Key Structure"))
  (bind _spinebonefollower (`self.SpineBoneFollower`))
  ;[1 1 1] When the left mouse button or space bar is pressed, set "Use Component Transform" to the opposite value of the current value.
  (:`Pressed`
    (if (`SpineBoneFollowerComponent.UseComponentTransform` (`self.SpineBoneFollower`)) :!label _label
      (set `SpineBoneFollowerComponent.UseComponentTransform` false _spinebonefollower)
      (`KismetSystemLibrary.PrintString` "Use Component Transform: False" true true (struct :`R` 0.09375 :`G` 0.341416 :`B` 1.0 :`A` 1.0) 1.0)
      (else
        (set `SpineBoneFollowerComponent.UseComponentTransform` true _spinebonefollower)
        (`KismetSystemLibrary.PrintString` "Use Component Transform: True" true true (struct :`R` 0.052192 :`G` 0.770833 :`B` 0.252641 :`A` 1.0) 1.0)))))

(event `Key|SpaceBar`
  (params (Key :type "Key Structure"))
  ;[1 1 1] When the left mouse button or space bar is pressed, set "Use Component Transform" to the opposite value of the current value.
  (:`Pressed`
    (goto _label)))

(fn `UserConstructionScript`)