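; Raptor demo Blueprint that drives a Spine skeleton animation with layered tracks and event callbacks.
; On BeginPlay, track 0 loops the walk animation and plays a 2D footstep sound whenever its "footstep" event fires.
; Track 1 plays gun-grab, queues gun-holster after a delay, and restarts that sequence each time the holster completes, creating an endless loop over the walk.
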(event `self.ReceiveBeginPlay`
  (bind _spineskeletonanimation (`self.SpineSkeletonAnimation`))
  ;[1 1 1] Loop the walk animation on track 0
  (bind _returnvalue (`SpineSkeletonAnimationComponent.SetAnimation` (`self.SpineSkeletonAnimation`) 0 "walk" true))
  ;[1 1 1] Bind to the custom animation event. If we get a user defined event
  ; called "footstep", playback the foot step sound"
  (add `TrackEntry.AnimationEvent` _returnvalue (delegate `AnimationEvent_Event_0`))
  ;[1 1 1] On track 1, we queue the gun-grab and gun-holster animations, the latter having a delay
  ; of 2 seconds. We listen for the completion of the gun-holster animation and start the
  ; sequence from the beginning.
  (`SpineSkeletonAnimationComponent.SetAnimation` _spineskeletonanimation 1 "gun-grab" false :!label _label)
  (bind _returnvalue_2 (`SpineSkeletonAnimationComponent.AddAnimation` _spineskeletonanimation 1 "gun-holster" false 2.0))
  (add `TrackEntry.AnimationComplete` _returnvalue_2 (delegate `AnimationComplete_Event_0`)))

(event `AnimationEvent_Event_0`
  (params (entry :type "TrackEntry Object Reference") (evt :type "SpineEvent Structure"))
  ;[1 1 1] Bind to the custom animation event. If we get a user defined event
  ; called "footstep", playback the foot step sound"
  (if (`KismetStringLibrary.EqualEqual_StrStr` (`.Name` (break `SpineEvent` evt)) "footstep")
    (`GameplayStatics.PlaySound2D` "/Game/GettingStarted/Assets/Sounds/Footstep.Footstep" 1.0 1.0 0.0 null null)))

(event `AnimationComplete_Event_0`
  (params (entry :type "TrackEntry Object Reference"))
  ;[1 1 1] On track 1, we queue the gun-grab and gun-holster animations, the latter having a delay
  ; of 2 seconds. We listen for the completion of the gun-holster animation and start the
  ; sequence from the beginning.
  (goto _label))

(fn `UserConstructionScript`)