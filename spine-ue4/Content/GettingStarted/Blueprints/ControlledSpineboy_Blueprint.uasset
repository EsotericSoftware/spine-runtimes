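; Spineboy example actor that shows keyboard-driven Spine skeletal animation.
; On BeginPlay it enables input for player 0 and loops the idle animation.
; H and K flip the skeleton's X scale and play run on track 0, returning to idle on release.
; Space layers a looping shoot on track 1 and blends it out with an empty animation on release, so shooting combines with running.
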(event `self.ReceiveBeginPlay`
  ;[1 1 1] Enable Input on the actor
  (`self.EnableInput` (`GameplayStatics.GetPlayerController` 0))
  (`SpineSkeletonAnimationComponent.SetAnimation` (`self.SpineSkeletonAnimation`) 0 "idle" true))

(event `Key|H`
  (params (Key :type "Key Structure"))
  ;[1 1 1] React to 'H' key, letting Spineboy run to the left, and changing back to idle
  ; If we no longer press the key
  (:`Pressed`
    (`SpineSkeletonComponent.SetScaleX` (`self.SpineSkeletonAnimation`) -1.0)
    (`SpineSkeletonAnimationComponent.SetAnimation` (`self.SpineSkeletonAnimation`) 0 "run" true))
  (:`Released`
    (`SpineSkeletonAnimationComponent.SetAnimation` (`self.SpineSkeletonAnimation`) 0 "idle" true)))

(event `Key|K`
  (params (Key :type "Key Structure"))
  ;[1 1 1] React to 'K' key, letting Spineboy run to the right, and changing back to idle
  ; If we no longer press the key
  (:`Pressed`
    (`SpineSkeletonComponent.SetScaleX` (`self.SpineSkeletonAnimation`) 1.0)
    (`SpineSkeletonAnimationComponent.SetAnimation` (`self.SpineSkeletonAnimation`) 0 "run" true))
  (:`Released`
    (`SpineSkeletonAnimationComponent.SetAnimation` (`self.SpineSkeletonAnimation`) 0 "idle" true)))

(event `Key|SpaceBar`
  (params (Key :type "Key Structure"))
  ;[1 1 1] React to 'SPACE' key, let Spineboy shoot  on track 1 while running
  (:`Pressed`
    (`SpineSkeletonAnimationComponent.SetAnimation` (`self.SpineSkeletonAnimation`) 1 "shoot" true))
  (:`Released`
    (`SpineSkeletonAnimationComponent.SetEmptyAnimation` (`self.SpineSkeletonAnimation`) 1 0.2)))

(fn `UserConstructionScript`)