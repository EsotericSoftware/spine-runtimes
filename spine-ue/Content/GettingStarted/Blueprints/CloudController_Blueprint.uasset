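; Cloud controller actor from the Getting Started content that lets the player steer a Spine skeleton's "cloud" bone with the keyboard.
; Each Tick it polls the U, J, H and K keys on player controller 0 and offsets its root component along world Z or X at a fixed, frame-rate-independent speed.
; Per the graph comment, a SpineBoneDriver on the actor then moves the bone to the actor's location.
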(event `self.ReceiveTick`
  (params (DeltaSeconds :type "Float (single-precision)"))
  (bind _returnvalue (`GameplayStatics.GetPlayerController` 0))
  (bind _returnvalue_2 (* DeltaSeconds 1400.0))
  (bind _defaultsceneroot1 (`self.DefaultSceneRoot1`))
  (bind _defaultsceneroot1_2 (`self.DefaultSceneRoot1`))
  ;[1 1 1] Move the actor every tick depending on which of the U/H/J/K keys are pressed. The SpineBoneDriver on that actor will then move the "cloud" bone in the skeleton to that actor's location.
  (`|ExecutionSequence`
    (:`then_0`
      (if (> (`PlayerController.GetInputKeyTimeDown` _returnvalue "U") 0.0)
        (`SceneComponent.K2_AddWorldOffset` _defaultsceneroot1 (`KismetMathLibrary.MakeVector` 0.0 0.0 _returnvalue_2) false false)))
    (:`then_1`
      (if (> (`PlayerController.GetInputKeyTimeDown` _returnvalue "J") 0.0)
        (`SceneComponent.K2_AddWorldOffset` _defaultsceneroot1 (`KismetMathLibrary.MakeVector` 0.0 0.0 (* _returnvalue_2 -1.0)) false false)))
    (:`then_2`
      (if (> (`PlayerController.GetInputKeyTimeDown` _returnvalue "K") 0.0)
        (`SceneComponent.K2_AddWorldOffset` _defaultsceneroot1_2 (`KismetMathLibrary.MakeVector` _returnvalue_2) false false)))
    (:`then_3`
      (if (> (`PlayerController.GetInputKeyTimeDown` _returnvalue "H") 0.0)
        (`SceneComponent.K2_AddWorldOffset` _defaultsceneroot1_2 (`KismetMathLibrary.MakeVector` (* _returnvalue_2 -1.0)) false false)))))

(fn `UserConstructionScript`)