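; Spine example actor that toggles a 2D skeletal character between a boy skin and a girl skin at runtime.
; On BeginPlay it applies the boy skin, loops a walk animation on track 0 and enables player input.
; Left click or spacebar flips the IsGirl flag, applying either one prebuilt boy skin or a girl look combined from multiple part skins via SetSkins, then resets slots to setup pose.
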(event `Key|LeftMouseButton`
  (params (Key :type "Key Structure"))
  (bind _spineskeletonanimation (`self.SpineSkeletonAnimation`))
  ;[1 1 1] Left click or  press spacebar to switch between the boy skin and the girl skin. The girl's skin has been set by combining multiple skins.
  (:`Pressed`
    (if (`self.IsGirl`) :!label _label
      (`SpineSkeletonComponent.SetSkin` _spineskeletonanimation "full-skins/boy")
      (`SpineSkeletonComponent.SetSlotsToSetupPose` _spineskeletonanimation)
      (set `self.IsGirl` false)
      (else
        (`SpineSkeletonComponent.SetSkins` _spineskeletonanimation (`|MakeArray` "skin-base" "accessories/bag" "eyelids/girly" "hair/long-blue-with-scarf" "legs/boots-red" "nose/short" "eyes/eyes-blue" "accessories/scarf" "accessories/hat-pointy-blue-yellow" "legs/pants-jeans" "clothes/hoodie-blue-and-scarf"))
        (`SpineSkeletonComponent.SetSlotsToSetupPose` _spineskeletonanimation)
        (set `self.IsGirl` true)))))

(event `self.ReceiveBeginPlay`
  (bind _spineskeletonanimation (`self.SpineSkeletonAnimation`))
  ;[1 1 1] Set the initial skin and walk animation to track 0 , then enable the input.
  (`SpineSkeletonComponent.SetSkin` _spineskeletonanimation "full-skins/boy")
  (`SpineSkeletonAnimationComponent.SetAnimation` _spineskeletonanimation 0 "walk" true)
  (`self.EnableInput` (`GameplayStatics.GetPlayerController` 0)))

(event `Key|SpaceBar`
  (params (Key :type "Key Structure"))
  ;[1 1 1] Left click or  press spacebar to switch between the boy skin and the girl skin. The girl's skin has been set by combining multiple skins.
  (:`Pressed`
    (goto _label)))

(fn `UserConstructionScript`)